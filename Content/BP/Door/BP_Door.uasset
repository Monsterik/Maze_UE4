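; BP_Door is a swinging door the player uses, and it can be flagged as the winning door.
; A trigger outlines a closed, non-first door via custom depth stencil and arms the player's use event through DoOnce and Gate nodes.
; Using it passes the door to BP_GameState and calls Win on the player for a win door.
; Timelines animate yaw while collision toggles, and a GameState event is bound for closing doors.
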(event OnComponentBeginOverlap(Trigger)
  (params (OverlappedComponent :type Primitive%20Component%20Object%20Reference) (OtherActor :type Actor%20Object%20Reference) (OtherComp :type Primitive%20Component%20Object%20Reference) (OtherBodyIndex :type Integer) (bFromSweep :type Boolean) (SweepResult :type Hit%20Result%20Structure%20%28by%20ref%29))
  ;[1 1 1] Control door availability
  (Utilities|Casting|CastToBP_PlayerCharacter OtherActor)
  (if (and (not (Variables|Default|GetOpen)) (not (Variables|Default|GetFirstDoor)))
    (CallFunction|ChangeOutline true)
    (Utilities|FlowControl|Sequence
      (:then_0
        (Utilities|FlowControl|DoOnce false) ; enters at Reset
      )
      (:then_1
        (Utilities|FlowControl|Gate true) ; enters at Open
      ))))

(event OnComponentEndOverlap(Trigger)
  (params (OverlappedComponent :type Primitive%20Component%20Object%20Reference) (OtherActor :type Actor%20Object%20Reference) (OtherComp :type Primitive%20Component%20Object%20Reference) (OtherBodyIndex :type Integer))
  ;[1 1 1] Control door availability
  (Utilities|Casting|CastToBP_PlayerCharacter OtherActor)
  (CallFunction|ChangeOutline false)
  (Utilities|FlowControl|Gate true) ; enters at Close
)

(event Custom|Use%20Door
  ;[1 1 1] Control door availability
  (Utilities|FlowControl|DoOnce false
    (:Completed
      (Utilities|FlowControl|Gate true
        (:Exit
          ;[1 1 1] Door opening
          (bind _asbp_game_state (Utilities|Casting|CastToBP_GameState (Game|GetGameState)))
          (Default|OpenDoor _asbp_game_state self)
          (CallFunction|ChangeOutline false)
          ;[1 1 1] Check if player win
          (if (Variables|Default|GetWinDoor)
            (bind _asbp_player_character (Utilities|Casting|CastToBP_PlayerCharacter (Game|GetPlayerCharacter 0)))
            (Default|Win _asbp_player_character)))))))

(event Custom|Close%20Opened%20Doors
  ;[1 1 1] Close Opened Doors
  (if (Variables|Default|GetOpen)
    (Variables|Default|SetOpen false)
    (bind _z_rotator (Timeline|Close%20Timeline PlayFromStart)
      (:Update
        (Transformation|SetRelativeRotation (Variables|Default|GetSM_Door) (Math|Rotator|MakeRotator 0.0 0.0 _z_rotator) false false))
      (:Finished
        (Collision|SetCollisionEnabled (Variables|Default|GetSM_Door) "QueryAndPhysics")))))

(event Custom|Open%20Door
  ;[1 1 1] Open Door
  (Variables|Default|SetOpen true)
  (Collision|SetCollisionEnabled (Variables|Default|GetSM_Door) "NoCollision")
  (bind _z_rotator (Timeline|Open%20Timeline PlayFromStart)
    (:Update
      (Transformation|SetRelativeRotation (Variables|Default|GetSM_Door) (Math|Rotator|MakeRotator 0.0 0.0 _z_rotator) false false))))

(event EventBeginPlay
  ;[1 1 1] Bind use door
  (bind _asbp_player_character (Utilities|Casting|CastToBP_PlayerCharacter (Game|GetPlayerCharacter 0)))
  (EventDispatchers|BindEventtoUseDoor _asbp_player_character (EventDispatchers|CreateEvent :!event Custom|Use%20Door))
  ;[1 1 1] Bind close event
  (bind _asbp_game_state (Utilities|Casting|CastToBP_GameState (Game|GetGameState)))
  (EventDispatchers|BindEventtoCloseDoors _asbp_game_state (EventDispatchers|CreateEvent :!event Custom|Close%20Opened%20Doors))
  ;[1 1 1] Doors that should be open at the begin play are made open
  (if (Variables|Default|GetOpen)
    (Transformation|SetRelativeRotation (Variables|Default|GetSM_Door) (Math|Rotator|MakeRotator 0.0 0.0 9e+01) false false)
    (Collision|SetCollisionEnabled (Variables|Default|GetSM_Door) "NoCollision")))

(fn ConstructionScript)

(fn ChangeOutline
  (params (Active :type Boolean))
  (bind _sm_door (Variables|Default|GetSM_Door))
  (bind _sm_door_2 (Variables|Default|GetSM_Door))
  (if Active
    (Rendering|SetRenderCustomDepth _sm_door true)
    (Rendering|SetCustomDepthStencilValue _sm_door 2)
    (else
      (Rendering|SetRenderCustomDepth _sm_door_2 false)
      (Rendering|SetCustomDepthStencilValue _sm_door_2 0))))