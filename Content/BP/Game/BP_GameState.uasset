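; Game state that runs a room-and-door chase between player and enemy, opening a door on request or randomly when a timer expires.
; Overlap tests locate both characters' rooms; each move closes doors, opens the player's door and restarts the timer.
; Unless that door links to the enemy's room, a random eligible enemy door also opens.
; The enemy's Blackboard RoomCenter then receives the new room's location.
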(event Custom|Auto%20Open%20Random%20Door
  ;[1 1 1] Auto Open Random Door
  (Variables|Default|SetAuto true)
  (bind _player_room (CallFunction|GetPlayerRoom))
  (bind _enemy_room (CallFunction|GetEnemyRoom))
  (if (Variables|Default|GetAuto)
    (bind _door (CallFunction|ChooseRandomConnectedDoor _player_room))
    (Variables|Default|SetPlayerDoor _door))
  (bind _true (CallFunction|IfOpenedDoortoEnemy _player_room (Variables|Default|GetPlayerDoor) _enemy_room))
  (if _true
    (Default|CallCloseDoors)
    (Default|OpenDoor (Variables|Default|GetPlayerDoor))
    (CallFunction|ResetTimer)
    (else
      (bind (_door_2 _random_room_for_enemy) (CallFunction|ChooseRandomConnectedDoor _enemy_room))
      (Default|CallCloseDoors)
      (Default|OpenDoor (Variables|Default|GetPlayerDoor))
      (Default|OpenDoor _door_2)
      (CallFunction|MoveEnemytoNewRoom _random_room_for_enemy)
      (CallFunction|ResetTimer))))

(event Custom|Reset%20Timer
  ;[1 1 1] Set and reset timer
  (bind _returnvalue (Utilities|Time|SetTimerbyEvent (delegate Custom|Auto%20Open%20Random%20Door) (Variables|Default|GetTimerInSeconds)))
  (Variables|Default|SetTimer _returnvalue))

(event Custom|Open%20Door
  (params (Door :type BP%20Door%20Object%20Reference))
  ;[1 1 1] Auto Open Random Door
  (Variables|Default|SetPlayerDoor Door)
  (Variables|Default|SetAuto false)
  (bind _player_room (CallFunction|GetPlayerRoom))
  (bind _enemy_room (CallFunction|GetEnemyRoom))
  (if (Variables|Default|GetAuto)
    (bind _door (CallFunction|ChooseRandomConnectedDoor _player_room))
    (Variables|Default|SetPlayerDoor _door))
  (bind _true (CallFunction|IfOpenedDoortoEnemy _player_room (Variables|Default|GetPlayerDoor) _enemy_room))
  (if _true
    (Default|CallCloseDoors)
    (Default|OpenDoor (Variables|Default|GetPlayerDoor))
    (CallFunction|ResetTimer)
    (else
      (bind (_door_2 _random_room_for_enemy) (CallFunction|ChooseRandomConnectedDoor _enemy_room))
      (Default|CallCloseDoors)
      (Default|OpenDoor (Variables|Default|GetPlayerDoor))
      (Default|OpenDoor _door_2)
      (CallFunction|MoveEnemytoNewRoom _random_room_for_enemy)
      (CallFunction|ResetTimer))))

(event EventBeginPlay
  ;[1 1 1] Get all doors for auto opening
  (bind _outactors (Actor|GetAllActorsOfClass "/Game/BP/Door/BP_Door.BP_Door_C"))
  (Variables|Default|SetDoors _outactors))

(fn ConstructionScript)

(fn GetPlayerRoom
  (for _array_element (Variables|Default|GetRooms)
    (if (Collision|IsOverlappingActor (Utilities|ResolveSoftReference _array_element) (Game|GetPlayerCharacter 0) :!class /Script/Engine.Actor)
      (return (Utilities|ResolveSoftReference _array_element)))))

(fn ChooseRandomConnectedDoor
  (params (Current%20Room :type Trigger%20Box%20Object%20Reference))
  (bind _doorstochoosefrom (Variables|Default|GetDoorsToChooseFrom))
  (for _array_element (Variables|Default|GetDoors)
    (for _array_element_2 (Variables|/Game/BP/Door/BP_Door.BP_Door_C|GetConnectedRooms _array_element)
      (if (Math|Boolean|ANDBoolean (== (Utilities|ResolveSoftReference _array_element_2) Current%20Room) (not (Variables|/Game/BP/Door/BP_Door.BP_Door_C|GetOpen _array_element)) (not (Variables|/Game/BP/Door/BP_Door.BP_Door_C|GetWinDoor _array_element)) (not (Variables|/Game/BP/Door/BP_Door.BP_Door_C|GetFirstDoor _array_element)))
        (Utilities|Array|Add (Variables|Default|GetDoorsToChooseFrom) _array_element))))
  (LocalVariables|SetRandomDoor (Utilities|Array|Get(acopy) _doorstochoosefrom (Math|Random|RandomIntegerinRange 0 (- (Utilities|Array|Length _doorstochoosefrom) 1))))
  (Utilities|Array|Clear (Variables|Default|GetDoorsToChooseFrom))
  (return (LocalVariables|GetRandomDoor) (select (== Current%20Room (Utilities|ResolveSoftReference (Utilities|Array|Get(acopy) (Variables|/Game/BP/Door/BP_Door.BP_Door_C|GetConnectedRooms (LocalVariables|GetRandomDoor))))) (Utilities|ResolveSoftReference (Utilities|Array|Get(acopy) (Variables|/Game/BP/Door/BP_Door.BP_Door_C|GetConnectedRooms (LocalVariables|GetRandomDoor)) 1)) (Utilities|ResolveSoftReference (Utilities|Array|Get(acopy) (Variables|/Game/BP/Door/BP_Door.BP_Door_C|GetConnectedRooms (LocalVariables|GetRandomDoor)))))))

(fn GetEnemyRoom
  (for _array_element (Variables|Default|GetRooms)
    (if (Collision|IsOverlappingActor (Utilities|ResolveSoftReference _array_element) (Utilities|ResolveSoftReference (Variables|Default|GetEnemy)) :!class /Script/Engine.Actor)
      (return (Utilities|ResolveSoftReference _array_element)))))

(fn MoveEnemytoNewRoom
  (params (Room :type Trigger%20Box%20Object%20Reference))
  (AI|Components|Blackboard|SetValueasVector (AI|GetBlackboard (AI|GetAIController (Utilities|ResolveSoftReference (Variables|Default|GetEnemy)))) (Utilities|Name|MakeLiteralName "RoomCenter") (Transformation|GetActorLocation Room)))

(fn IfOpenedDoortoEnemy
  (params (Player%20Room :type Trigger%20Box%20Object%20Reference) (Player%20Door :type BP%20Door%20Object%20Reference) (Enemy%20Room :type Trigger%20Box%20Object%20Reference))
  (bind _connectedrooms (Variables|/Game/BP/Door/BP_Door.BP_Door_C|GetConnectedRooms Player%20Door))
  (bind _output (Utilities|Array|Get(acopy) _connectedrooms))
  (bind _output_2 (Utilities|Array|Get(acopy) _connectedrooms 1))
  (bind _output_3 (Utilities|ResolveSoftReference _output_2))
  (bind _output_4 (Utilities|ResolveSoftReference _output))
  (if (or (and (== Player%20Room _output_4) (== _output_3 Enemy%20Room)) (and (== Player%20Room _output_3) (== _output_4 Enemy%20Room)))
    (return true)
    (else
      (return false))))